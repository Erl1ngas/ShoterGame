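; BP_MasterITem is a pickup item that registers with the inventory component of actors overlapping its interaction collision.
; With AutoActivate on that component, the item adds itself and is destroyed.
; Otherwise it becomes the pickup candidate and shows the interaction indicator, which hides on exit when no overlapping items remain.
; Construction either enables mesh physics or, without physics, removes rotating movement unless it is enabled.
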(event OnComponentBeginOverlap(InteractColl)
  (params (OverlappedComponent :type Primitive%20Component%20Object%20Reference) (OtherActor :type Actor%20Object%20Reference) (OtherComp :type Primitive%20Component%20Object%20Reference) (OtherBodyIndex :type Integer) (bFromSweep :type Boolean) (SweepResult :type Hit%20Result%20Structure%20%28by%20ref%29))
  (bind _returnvalue (Actor|GetComponentbyClass OtherActor "/Game/CrazyPeople/Estructures/AC_InventoryComponent.AC_InventoryComponent_C"))
  (if (Utilities|DoesObjectImplementInterface _returnvalue "/Game/CrazyPeople/Estructures/BPI_InventoryInterface.BPI_InventoryInterface_C")
    (if (Variables|/Script/Engine.ActorComponent|GetbAutoActivate _returnvalue)
      (Default|FAddItemtoInventory _returnvalue self)
      (Actor|DestroyActor)
      (else
        (Utilities|Array|Add (Variables|/Game/CrazyPeople/Estructures/AC_InventoryComponent.AC_InventoryComponent_C|GetOverlappingItems _returnvalue) self)
        (Variables|/Game/CrazyPeople/Estructures/AC_InventoryComponent.AC_InventoryComponent_C|SetItemToPickup _returnvalue self)
        (Default|SetInteractionVisibility _returnvalue true)))))

(event OnComponentEndOverlap(InteractColl)
  (params (OverlappedComponent :type Primitive%20Component%20Object%20Reference) (OtherActor :type Actor%20Object%20Reference) (OtherComp :type Primitive%20Component%20Object%20Reference) (OtherBodyIndex :type Integer))
  (bind _returnvalue (Actor|GetComponentbyClass OtherActor "/Game/CrazyPeople/Estructures/AC_InventoryComponent.AC_InventoryComponent_C"))
  (bind _overlappingitems (Variables|/Game/CrazyPeople/Estructures/AC_InventoryComponent.AC_InventoryComponent_C|GetOverlappingItems _returnvalue))
  (Utilities|IsValid OtherActor
    (:Is%20Valid
      (if (Utilities|DoesObjectImplementInterface _returnvalue "/Game/CrazyPeople/Estructures/BPI_InventoryInterface.BPI_InventoryInterface_C")
        (Utilities|Array|RemoveItem _overlappingitems self)
        (if (not (> (Utilities|Array|Length _overlappingitems) 0))
          (Default|SetInteractionVisibility _returnvalue false))))))

(fn ConstructionScript
  (if (Variables|Default|GetUsePhysics)
    (Physics|SetSimulatePhysics (Variables|Default|GetStaticMesh) true)
    (Collision|SetCollisionEnabled (Variables|Default|GetStaticMesh) "QueryAndPhysics")
    (elif (not (Variables|Default|GetUseRotatingMovement))
      (Components|DestroyComponent (Variables|Default|GetRotatingMovement)))))