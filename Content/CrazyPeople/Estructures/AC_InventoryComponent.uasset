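; Multiplayer inventory component for the CrazyPeople character, handling item pickup, stack drops, weapon and health-potion slots, and potion use.
; Items are stored as a class array with one entry per stacked unit, with item data read from class defaults.
; Server events handle spawning, destruction and slot changes, while OnReps attach three runtime-created weapon meshes to sockets and set pose indices on weapon switches.
; It also drives inventory, drop-amount, interaction and HUD widgets.
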(event Custom|Server_SpawnItem
  (params (Class :type Actor%20Class%20Reference) (SpawnTransform :type Transform) (CurrentStack :type Integer))
  ;[0.07338 1 0.01239] Spawn Item
  (bind _returnvalue (Game|SpawnActorfromClass Class SpawnTransform "Undefined" 0 0))
  (bind _asbp_third_person_character_crazy_people (Utilities|Casting|CastToBP_ThirdPersonCharacter_CrazyPeople _returnvalue))
  (Variables|/Game/CrazyPeople/BluePrint/BP_ThirdPersonCharacter_CrazyPeople.BP_ThirdPersonCharacter_CrazyPeople_C|SetCurrentStack _asbp_third_person_character_crazy_people CurrentStack))

(event Custom|Cliet_SpawnItem
  (params (Class :type Actor%20Class%20Reference) (SpawnTransform :type Transform))
  ;[0.07338 1 0.01239] Spawn Item
)

(event Custom|Server_SetMeleWeapon
  (params (EquippedMele :type BP%20Master%20I%20Tem%20Class%20Reference))
  ;[0 1 0.07465] Set Equippment
  (Variables|Default|SetEquippedMele EquippedMele))

(event Custom|Set_PrimaryWeaponEquipped
  (params (WeaponEquipped :type Boolean))
  ;[0 1 0.07465] Set Equippment
  (Variables|Default|SetWeaponEquipped WeaponEquipped))

(event Custom|Set_SecondaryWeaponEquipped
  (params (SecondaryEquipped :type Boolean))
  ;[0 1 0.07465] Set Equippment
  (Variables|Default|SetSecondaryEquipped SecondaryEquipped))

(event Custom|Set_MeleEquipped
  (params (MeleEquipped :type Boolean))
  ;[0 1 0.07465] Set Equippment
  (Variables|Default|SetMeleEquipped MeleEquipped))

(event Custom|SwitchPrimaryWeapon
  (params (SwitchPrimary :type Boolean))
  ;[1 1 1] Swithc Equipment
  (Variables|Default|SetSwitchPrimary SwitchPrimary))

(event Custom|Use_HelthPotion
  (bind _equippedhealth (Variables|Default|GetEquippedHealth))
  (bind (_itemname _description _itemimage _itemmesh _usephysics _userotatingmovement _maxstack _currentstack _itemtype _equipsocket _uneequippedsocket _consumabletype _consumablemodifier) (Utilities|GetClassDefaults _equippedhealth))
  ;[0.008445 0.6859 1] HealthPotion Funtion
  (switch Utilities|FlowControl|Switch|SwitchonE_ConsumableType _consumabletype
    (:NewEnumerator1
      (bind _asbp_third_person_character_crazy_people (Utilities|Casting|CastToBP_ThirdPersonCharacter_CrazyPeople (Variables|Default|GetOwningActor)))
      (bind _output_get (Variables|/Game/CrazyPeople/BluePrint/BP_ThirdPersonCharacter_CrazyPeople.BP_ThirdPersonCharacter_CrazyPeople_C|SetHealth _asbp_third_person_character_crazy_people (+ (Variables|/Game/CrazyPeople/BluePrint/BP_ThirdPersonCharacter_CrazyPeople.BP_ThirdPersonCharacter_CrazyPeople_C|GetHealth _asbp_third_person_character_crazy_people) _consumablemodifier)))
      (Development|PrintString (Utilities|String|ToString(Float) _output_get))
      (bind _outofstock (CallFunction|FRemoveItem (Variables|Default|GetEquippedHealth)))
      (CallFunction|FUpdateInventory)
      (if _outofstock
        (CallFunction|ServerSetHelthPotion "/Game/CrazyPeople/Estructures/BP_EmptyHolderItem.BP_EmptyHolderItem_C")
        (Default|FUpdate (Variables|/Game/CrazyPeople/WidgedBlueprint/WB_Inventory.WB_Inventory_C|GetWB_HealthSlot (Variables|Default|GetWB_Inventory)) "/Game/CrazyPeople/Estructures/BP_EmptyHolderItem.BP_EmptyHolderItem_C")
        (bind _asbp_third_person_character_crazy_people_2 (Utilities|Casting|CastToBP_ThirdPersonCharacter_CrazyPeople (Components|GetOwner)))
        (Default|UpdateConsumable (Variables|/Game/CrazyPeople/BluePrint/BP_ThirdPersonCharacter_CrazyPeople.BP_ThirdPersonCharacter_CrazyPeople_C|GetPlayerHudReference _asbp_third_person_character_crazy_people_2) "/Game/CrazyPeople/Estructures/BP_EmptyHolderItem.BP_EmptyHolderItem_C")
        (Widget|SetVisibility (Variables|/Game/CrazyPeople/WidgedBlueprint/WB_Hud.WB_Hud_C|GetItemAmount (Variables|/Game/CrazyPeople/BluePrint/BP_ThirdPersonCharacter_CrazyPeople.BP_ThirdPersonCharacter_CrazyPeople_C|GetPlayerHudReference _asbp_third_person_character_crazy_people_2)) "Collapsed")
        (else
          (bind _asbp_third_person_character_crazy_people_3 (Utilities|Casting|CastToBP_ThirdPersonCharacter_CrazyPeople (Components|GetOwner)))
          (Default|UpdateConsumable (Variables|/Game/CrazyPeople/BluePrint/BP_ThirdPersonCharacter_CrazyPeople.BP_ThirdPersonCharacter_CrazyPeople_C|GetPlayerHudReference _asbp_third_person_character_crazy_people_3) (Variables|Default|GetEquippedHealth)))))))

(event Custom|SwitchSecondaryWeapon
  (params (SwichtSecondary :type Boolean))
  ;[1 1 1] Swithc Equipment
  (Variables|Default|SetSwichtSecondary SwichtSecondary))

(event Custom|SwichtMele
  (params (SwitchMele :type Boolean))
  ;[1 1 1] Swithc Equipment
  (Variables|Default|SetSwitchMele SwitchMele))

(event Custom|Client_Aim
  (params (IsAiming? :type Boolean))
  (CallFunction|ServerSetIsAiming IsAiming?))

(event Custom|Server_SetIsAiming
  (params (IsAiming? :type Boolean))
  (Variables|Default|SetIsAiming? IsAiming?))

(event Custom|Server_PlaySound
  (params (Location :type Vector) (Sound :type Sound%20Base%20Object%20Reference))
  ;[0.03694 1 0] Sound Of PickUp
  (CallFunction|MCPlaySound Location Sound))

(event Custom|MC_PlaySound
  (params (Location :type Vector) (Sound :type Sound%20Base%20Object%20Reference))
  ;[0.03694 1 0] Sound Of PickUp
  (Audio|PlaySoundatLocation Sound Location "0, 0, 0" 1.0 1.0 0.0 0 0 0 0))

(event Custom|Server_DestroyActor
  (params (ActorToDestroy :type Actor%20Object%20Reference))
  ;[0.07338 1 0.01239] Spawn Item
  (Actor|DestroyActor ActorToDestroy))

(event Custom|Server_SetPrimaryWeapon
  (params (EquippedPrimary :type BP%20Master%20I%20Tem%20Class%20Reference))
  ;[0 1 0.07465] Set Equippment
  (Variables|Default|SetEquippedPrimary EquippedPrimary))

(event Custom|Initiate
  (params (OwningActor :type Actor%20Object%20Reference))
  ;[1 1 1] Iniciate Funtion
  (Utilities|FlowControl|Sequence
    (:then_0
      (bind _output_get (Variables|Default|SetOwningActor OwningActor))
      (bind _returnvalue (Game|AddComponentbyClass _output_get "/Script/Engine.StaticMeshComponent" false))
      (Variables|Default|SetPrimaryMesh _returnvalue)
      (bind _asbp_third_person_character_crazy_people (Utilities|Casting|CastToBP_ThirdPersonCharacter_CrazyPeople (Components|GetOwner)))
      (Variables|Default|SetHudReference (Variables|/Game/CrazyPeople/BluePrint/BP_ThirdPersonCharacter_CrazyPeople.BP_ThirdPersonCharacter_CrazyPeople_C|GetPlayerHudReference _asbp_third_person_character_crazy_people)))
    (:then_1
      (bind _returnvalue_2 (Game|AddComponentbyClass _output_get "/Script/Engine.StaticMeshComponent" false))
      (Variables|Default|SetSecondaryMesh _returnvalue_2))
    (:then_2
      (bind _returnvalue_3 (Game|AddComponentbyClass _output_get "/Script/Engine.StaticMeshComponent" false))
      (Variables|Default|SetMeleMesh _returnvalue_3))))

(event Custom|SetInteractionVisibility
  (params (Visible? :type Boolean))
  ;[1 1 1] Interaction Visibility "E"
  (if (Pawn|IsLocallyControlled (Variables|/Script/Engine.Actor|GetInstigator (Variables|Default|GetOwningActor)))
    (if Visible?
      (if (not (Variables|Default|GetInteractionVisible?))
        (Variables|Default|SetInteractionVisible? true)
        (bind _returnvalue (UserInterface|CreateWidget "/Game/CrazyPeople/WidgedBlueprint/WB_Interaction.WB_Interaction_C"))
        (bind _output_get (Variables|Default|SetWB_InteractionRef _returnvalue))
        (Utilities|IsValid _output_get
          (:Is%20Valid
            (UserInterface|Viewport|AddtoViewport _output_get 0))))
      (else
        (Utilities|IsValid (Variables|Default|GetWB_InteractionRef)
          (:Is%20Valid
            (Variables|Default|SetInteractionVisible? false)
            (Widget|RemovefromParent (Variables|Default|GetWB_InteractionRef))))))))

(event Custom|Server_SetSecondaryWeapon
  (params (EquippedSecondary :type BP%20Master%20I%20Tem%20Class%20Reference))
  ;[0 1 0.07465] Set Equippment
  (Variables|Default|SetEquippedSecondary EquippedSecondary))

(event Custom|Server_SetHelthPotion
  (params (EquippedHealth :type BP%20Master%20I%20Tem%20Class%20Reference))
  ;[0 1 0.07465] Set Equippment
  (Variables|Default|SetEquippedHealth EquippedHealth))

(event EventFSpawnItem
  (params (ItemToSpawn :type BP%20Master%20I%20Tem%20Class%20Reference) (SpawnTransform :type Transform))
  ;[0.07338 1 0.01239] Spawn Item
)

(fn FShowInventory
  (bind _returnvalue (Game|GetPlayerController 0))
  (if (and (not (Variables|Default|GetInventoryOpen?)) (Pawn|IsLocalPlayerController _returnvalue))
    (bind _returnvalue_2 (UserInterface|CreateWidget "/Game/CrazyPeople/WidgedBlueprint/WB_Inventory.WB_Inventory_C" _returnvalue))
    (Variables|Default|SetInventoryOpen? true)
    (bind _output_get (Variables|Default|SetWB_Inventory _returnvalue_2))
    (UserInterface|Viewport|AddtoViewport _output_get 0)
    (Default|FUpdate _returnvalue_2 "NewEnumerator0" (Variables|Default|GetEquippedSecondary) (Variables|Default|GetEquippedMele) (Variables|Default|GetEquippedHealth) (Variables|Default|GetEquippedPrimary))
    (if (not (Variables|Default|GetController))
      (Input|SetInputModeGameandUI (Game|GetPlayerController 0) (Variables|Default|GetWB_Inventory) "LockInFullscreen" true)
      (Variables|/Script/Engine.PlayerController|SetbShowMouseCursor (Game|GetPlayerController 0) true))))

(fn FHidenInventory
  (CallFunction|FRemoveItemAmountWidget)
  (Utilities|IsValid (Variables|Default|GetWB_Inventory)
    (:Is%20Valid
      (Widget|RemovefromParent (Variables|Default|GetWB_Inventory))
      (Variables|Default|SetInventoryOpen? false)
      (if (not (Variables|Default|GetController))
        (Input|SetInputModeGameOnly (Game|GetPlayerController 0))
        (Variables|/Script/Engine.PlayerController|SetbShowMouseCursor (Game|GetPlayerController 0) false)))))

(fn FAddItemtoInventory
  (params (ItemToAdd :type BP%20Master%20I%20Tem%20Object%20Reference))
  (bind _interactcoll (Variables|/Game/CrazyPeople/Estructures/BP_MasterITem.BP_MasterITem_C|GetInteractColl ItemToAdd))
  (bind _returnvalue (Transformation|GetWorldLocation _interactcoll))
  (Utilities|Array|Add (Variables|Default|GetInventory) (Utilities|GetClass ItemToAdd))
  (if (Variables|Default|GetInventoryOpen?)
    (CallFunction|FHidenInventory)
    (CallFunction|FShowInventory))
  (if (Variables|Default|GetReplicatedPickupSound)
    (Networking|SwitchHasAuthority
      (:Authority
        (CallFunction|MCPlaySound _returnvalue "/Engine/VREditor/Sounds/UI/Object_PickUp.Object_PickUp"))
      (:Remote
        (CallFunction|ServerPlaySound _returnvalue "/Engine/VREditor/Sounds/UI/Object_PickUp.Object_PickUp")))
    (else
      (Audio|PlaySound2D "/Engine/VREditor/Sounds/UI/Object_PickUp.Object_PickUp" 1.0 1.0 0.0 0 0))))

(fn FDropItem
  (params (ItemToSpawn :type BP%20Master%20I%20Tem%20Class%20Reference) (DropFromEquippementSlot :type Boolean) (CurrentStack :type Integer))
  (bind _inventory (Variables|Default|GetInventory))
  (LocalVariables|SetAmountToDrop CurrentStack)
  (LocalVariables|SetItemToDrop ItemToSpawn)
  (LocalVariables|SetDropPosition (Math|Conversions|ToTransform(Vector) (CallFunction|FUbicationOfDropItem)))
  (if DropFromEquippementSlot
    (switch Utilities|FlowControl|Switch|SwitchonE_ItemType (.ItemType (Utilities|GetClassDefaults (LocalVariables|GetItemToDrop)))
      (:NewEnumerator2
        (if (== (Variables|Default|GetEquippedPrimary) (LocalVariables|GetItemToDrop))
          (CallFunction|ServerSetPrimaryWeapon "/Game/CrazyPeople/Estructures/BP_EmptyHolderItem.BP_EmptyHolderItem_C")
          (Variables|Default|SetEquippedPrimary "/Game/CrazyPeople/Estructures/BP_EmptyHolderItem.BP_EmptyHolderItem_C")
          (CallFunction|ServerSpawnItem (LocalVariables|GetItemToDrop) (LocalVariables|GetDropPosition) 1 :!label _label)))
      (:NewEnumerator3
        (if (== (Variables|Default|GetEquippedSecondary) (LocalVariables|GetItemToDrop))
          (CallFunction|ServerSetSecondaryWeapon "/Game/CrazyPeople/Estructures/BP_EmptyHolderItem.BP_EmptyHolderItem_C")
          (Variables|Default|SetEquippedSecondary "/Game/CrazyPeople/Estructures/BP_EmptyHolderItem.BP_EmptyHolderItem_C")
          (goto _label)))
      (:NewEnumerator4
        (if (== (Variables|Default|GetEquippedHealth) (LocalVariables|GetItemToDrop))
          (CallFunction|ServerSetHelthPotion "/Game/CrazyPeople/Estructures/BP_EmptyHolderItem.BP_EmptyHolderItem_C")
          (Variables|Default|SetEquippedHealth "/Game/CrazyPeople/Estructures/BP_EmptyHolderItem.BP_EmptyHolderItem_C")
          (CallFunction|ResetHealthPotion)))
      (:NewEnumerator5
        (if (== (Variables|Default|GetEquippedMele) (LocalVariables|GetItemToDrop))
          (CallFunction|ServerSetMeleWeapon "/Game/CrazyPeople/Estructures/BP_EmptyHolderItem.BP_EmptyHolderItem_C")
          (Variables|Default|SetEquippedMele "/Game/CrazyPeople/Estructures/BP_EmptyHolderItem.BP_EmptyHolderItem_C")
          (goto _label))))
    (else
      (for _index (range 0 (LocalVariables|GetAmountToDrop))
        (Utilities|Array|RemoveIndex _inventory (Utilities|Array|FindItem _inventory (LocalVariables|GetItemToDrop))))
      (CallFunction|ServerSpawnItem (LocalVariables|GetItemToDrop) (LocalVariables|GetDropPosition) (LocalVariables|GetAmountToDrop))
      (if (== (Variables|Default|GetEquippedHealth) (LocalVariables|GetItemToDrop))
        (if (Utilities|Array|ContainsItem (Variables|Default|GetInventory) (LocalVariables|GetItemToDrop))
          (bind _asbp_third_person_character_crazy_people (Utilities|Casting|CastToBP_ThirdPersonCharacter_CrazyPeople (Components|GetOwner)))
          (Default|SetHudStackAmount (Variables|/Game/CrazyPeople/BluePrint/BP_ThirdPersonCharacter_CrazyPeople.BP_ThirdPersonCharacter_CrazyPeople_C|GetPlayerHudReference _asbp_third_person_character_crazy_people))
          (else
            (CallFunction|ServerSetHelthPotion "/Game/CrazyPeople/Estructures/BP_EmptyHolderItem.BP_EmptyHolderItem_C")
            (Variables|Default|SetEquippedHealth "/Game/CrazyPeople/Estructures/BP_EmptyHolderItem.BP_EmptyHolderItem_C")
            (bind _asbp_third_person_character_crazy_people_2 (Utilities|Casting|CastToBP_ThirdPersonCharacter_CrazyPeople (Components|GetOwner)))
            (Default|UpdateConsumable (Variables|/Game/CrazyPeople/BluePrint/BP_ThirdPersonCharacter_CrazyPeople.BP_ThirdPersonCharacter_CrazyPeople_C|GetPlayerHudReference _asbp_third_person_character_crazy_people_2) "/Game/CrazyPeople/Estructures/BP_EmptyHolderItem.BP_EmptyHolderItem_C")
            (Widget|SetVisibility (Variables|/Game/CrazyPeople/WidgedBlueprint/WB_Hud.WB_Hud_C|GetItemAmount (Variables|/Game/CrazyPeople/BluePrint/BP_ThirdPersonCharacter_CrazyPeople.BP_ThirdPersonCharacter_CrazyPeople_C|GetPlayerHudReference _asbp_third_person_character_crazy_people_2)) "Collapsed")))))))

(fn FTryPickupItem
  (bind _overlappingitems (Variables|Default|GetOverlappingItems))
  (if (> (Utilities|Array|Length (Variables|Default|GetOverlappingItems)) 0)
    (for _index (range 1 (Variables|/Game/CrazyPeople/Estructures/BP_MasterITem.BP_MasterITem_C|GetCurrentStack (Variables|Default|GetItemToPickup)))
      (CallFunction|FAddItemtoInventory (Variables|Default|GetItemToPickup)))
    (Utilities|Array|RemoveItem (Variables|Default|GetOverlappingItems) (Variables|Default|GetItemToPickup))
    (CallFunction|ServerDestroyActor (Variables|Default|GetItemToPickup))
    (if (> (Utilities|Array|Length _overlappingitems) 0)
      (Variables|Default|SetItemToPickup (.OutItem (Utilities|Array|Random _overlappingitems))))))

(fn FCreateItemAmountWidget
  (params (ItemToHandle :type BP%20Master%20I%20Tem%20Class%20Reference) (NumberInStack :type Integer))
  (CallFunction|FRemoveItemAmountWidget)
  (bind _returnvalue (UserInterface|CreateWidget "/Game/CrazyPeople/WidgedBlueprint/WB_ItemDropAmount.WB_ItemDropAmount_C" 0 (Variables|Default|GetInventory) ItemToHandle NumberInStack))
  (bind _output_get (Variables|Default|SetWB_ItemAmount _returnvalue))
  (UserInterface|Viewport|AddtoViewport _output_get 0)
  (bind _returnvalue_2 (Class|WidgetLayoutLibrary|GetMousePositiononViewport))
  (Class|UserWidget|SetPositioninViewport _output_get (Math|Vector2D|MakeVector2D (.x _returnvalue_2) (.y _returnvalue_2)) false))

(fn OnRepEquippedSecondary
  (bind _equippedsecondary (Variables|Default|GetEquippedSecondary))
  (bind (_itemname _description _itemimage _itemmesh _usephysics _userotatingmovement _maxstack _currentstack _itemtype _equipsocket _uneequippedsocket) (Utilities|GetClassDefaults _equippedsecondary))
  (bind _ascharacter (Utilities|Casting|CastToCharacter (Variables|Default|GetOwningActor)))
  (Transformation|AttachComponentToComponent (Variables|Default|GetSecondaryMesh) (Variables|/Script/Engine.Character|GetMesh _ascharacter) _uneequippedsocket "SnapToTarget" "SnapToTarget" "SnapToTarget" true)
  (Components|StaticMesh|SetStaticMesh (Variables|Default|GetSecondaryMesh) _itemmesh))

(fn OnRepEquippedMele
  (bind _equippedmele (Variables|Default|GetEquippedMele))
  (bind (_itemname _description _itemimage _itemmesh _usephysics _userotatingmovement _maxstack _currentstack _itemtype _equipsocket _uneequippedsocket) (Utilities|GetClassDefaults _equippedmele))
  (bind _ascharacter (Utilities|Casting|CastToCharacter (Variables|Default|GetOwningActor)))
  (Transformation|AttachComponentToComponent (Variables|Default|GetMeleMesh) (Variables|/Script/Engine.Character|GetMesh _ascharacter) _uneequippedsocket "SnapToTarget" "SnapToTarget" "SnapToTarget" true)
  (Components|StaticMesh|SetStaticMesh (Variables|Default|GetMeleMesh) _itemmesh))

(fn OnRepHolsteredWeapon)

(fn OnRepWeaponEquipped
  (if (Variables|Default|GetWeaponEquipped)
    (bind _ascharacter (Utilities|Casting|CastToCharacter (Variables|Default|GetOwningActor)))
    (Transformation|AttachComponentToComponent (Variables|Default|GetPrimaryMesh) (Variables|/Script/Engine.Character|GetMesh _ascharacter) (.EquipSocket (Utilities|GetClassDefaults (Variables|Default|GetEquippedPrimary))) "SnapToTarget" "SnapToTarget" "SnapToTarget" true)
    (else
      (bind _ascharacter_2 (Utilities|Casting|CastToCharacter (Variables|Default|GetOwningActor)))
      (Transformation|AttachComponentToComponent (Variables|Default|GetPrimaryMesh) (Variables|/Script/Engine.Character|GetMesh _ascharacter_2) (.UneEquippedSocket (Utilities|GetClassDefaults (Variables|Default|GetEquippedPrimary))) "SnapToTarget" "SnapToTarget" "SnapToTarget" true))))

(fn OnRepSecondaryEquipped
  (if (Variables|Default|GetSecondaryEquipped)
    (bind _ascharacter (Utilities|Casting|CastToCharacter (Variables|Default|GetOwningActor)))
    (Transformation|AttachComponentToComponent (Variables|Default|GetSecondaryMesh) (Variables|/Script/Engine.Character|GetMesh _ascharacter) (.EquipSocket (Utilities|GetClassDefaults (Variables|Default|GetEquippedSecondary))) "SnapToTarget" "SnapToTarget" "SnapToTarget" true)
    (else
      (bind _ascharacter_2 (Utilities|Casting|CastToCharacter (Variables|Default|GetOwningActor)))
      (Transformation|AttachComponentToComponent (Variables|Default|GetSecondaryMesh) (Variables|/Script/Engine.Character|GetMesh _ascharacter_2) (.UneEquippedSocket (Utilities|GetClassDefaults (Variables|Default|GetEquippedSecondary))) "SnapToTarget" "SnapToTarget" "SnapToTarget" true))))

(fn OnRepMeleEquipped
  (if (Variables|Default|GetMeleEquipped)
    (bind _ascharacter (Utilities|Casting|CastToCharacter (Variables|Default|GetOwningActor)))
    (Transformation|AttachComponentToComponent (Variables|Default|GetMeleMesh) (Variables|/Script/Engine.Character|GetMesh _ascharacter) (.EquipSocket (Utilities|GetClassDefaults (Variables|Default|GetEquippedMele))) "SnapToTarget" "SnapToTarget" "SnapToTarget" true)
    (else
      (bind _ascharacter_2 (Utilities|Casting|CastToCharacter (Variables|Default|GetOwningActor)))
      (Transformation|AttachComponentToComponent (Variables|Default|GetMeleMesh) (Variables|/Script/Engine.Character|GetMesh _ascharacter_2) (.UneEquippedSocket (Utilities|GetClassDefaults (Variables|Default|GetEquippedMele))) "SnapToTarget" "SnapToTarget" "SnapToTarget" true))))

(fn FDropHealthItem
  (params (ItemToRemove :type BP%20Master%20I%20Tem%20Class%20Reference))
  (bind _inventory (Variables|Default|GetInventory))
  (Utilities|Array|RemoveIndex _inventory (Utilities|Array|FindItem _inventory ItemToRemove)))

(fn HelperDropItem
  (bind _returnvalue (Components|GetOwner))
  (return (+ (+ (Transformation|GetActorLocation _returnvalue) (* (Math|Vector|GetForwardVector (Transformation|GetActorRotation _returnvalue)) (Variables|Default|GetItemToDistance))) (Math|Vector|MakeVector (Math|Random|RandomFloatinRange -75.0 75.0) (Math|Random|RandomFloatinRange -75.0 75.0) 0.0))))

(fn OnRepEquippedHealth)

(fn OnRepHealthEquipped)

(fn FRemoveItem
  (params (ItemToRemove :type BP%20Master%20I%20Tem%20Class%20Reference))
  (bind _inventory (Variables|Default|GetInventory))
  (bind _returnvalue (Utilities|Array|FindItem _inventory ItemToRemove))
  (Utilities|Array|RemoveIndex _inventory _returnvalue)
  (if (== _returnvalue -1)
    (return true)
    (else
      (return false))))

(fn FHelperDropItemTrace
  (bind _returnvalue (Components|GetOwner))
  (return (+ (+ (Transformation|GetActorLocation _returnvalue) (* (Math|Vector|GetForwardVector (Transformation|GetActorRotation _returnvalue)) (Variables|Default|GetItemToDistance))) (Math|Vector|MakeVector (Math|Random|RandomFloatinRange -75.0 75.0) (Math|Random|RandomFloatinRange -75.0 75.0) 0.0))))

(fn FUpdateInventory
  (if (Variables|Default|GetInventoryOpen?)
    (CallFunction|FHidenInventory)
    (CallFunction|FShowInventory)))

(fn FUbicationOfDropItem
  (bind _returnvalue (Components|GetOwner))
  (return (+ (+ (Transformation|GetActorLocation _returnvalue) (* (Math|Vector|GetForwardVector (Transformation|GetActorRotation _returnvalue)) (Variables|Default|GetItemToDistance))) (Math|Vector|MakeVector (Math|Random|RandomFloatinRange -75.0 75.0) (Math|Random|RandomFloatinRange -75.0 75.0) 0.0))))

(fn OnRepEquippedPrimary
  (bind _equippedprimary (Variables|Default|GetEquippedPrimary))
  (bind (_itemname _description _itemimage _itemmesh _usephysics _userotatingmovement _maxstack _currentstack _itemtype _equipsocket _uneequippedsocket) (Utilities|GetClassDefaults _equippedprimary))
  (bind _ascharacter (Utilities|Casting|CastToCharacter (Variables|Default|GetOwningActor)))
  (Transformation|AttachComponentToComponent (Variables|Default|GetPrimaryMesh) (Variables|/Script/Engine.Character|GetMesh _ascharacter) _uneequippedsocket "SnapToTarget" "SnapToTarget" "SnapToTarget" true)
  (Components|StaticMesh|SetStaticMesh (Variables|Default|GetPrimaryMesh) _itemmesh))

(fn FRemoveItemAmountWidget
  (Utilities|IsValid (Variables|Default|GetWB_ItemAmount)
    (:Is%20Valid
      (Widget|RemovefromParent (Variables|Default|GetWB_ItemAmount)))))

(fn ResetHealthPotion
  (bind _asbp_third_person_character_crazy_people (Utilities|Casting|CastToBP_ThirdPersonCharacter_CrazyPeople (Components|GetOwner)))
  (Default|UpdateConsumable (Variables|/Game/CrazyPeople/BluePrint/BP_ThirdPersonCharacter_CrazyPeople.BP_ThirdPersonCharacter_CrazyPeople_C|GetPlayerHudReference _asbp_third_person_character_crazy_people) "/Game/CrazyPeople/Estructures/BP_EmptyHolderItem.BP_EmptyHolderItem_C")
  (Widget|SetVisibility (Variables|/Game/CrazyPeople/WidgedBlueprint/WB_Hud.WB_Hud_C|GetItemAmount (Variables|/Game/CrazyPeople/BluePrint/BP_ThirdPersonCharacter_CrazyPeople.BP_ThirdPersonCharacter_CrazyPeople_C|GetPlayerHudReference _asbp_third_person_character_crazy_people)) "Collapsed"))

(fn OnRepSwitchPrimary
  (CallFunction|SetPrimaryWeaponEquipped true)
  (bind _asbp_third_person_character_crazy_people (Utilities|Casting|CastToBP_ThirdPersonCharacter_CrazyPeople (Variables|Default|GetOwningActor)))
  (Variables|/Game/CrazyPeople/BluePrint/BP_ThirdPersonCharacter_CrazyPeople.BP_ThirdPersonCharacter_CrazyPeople_C|SetTopPoseIndex _asbp_third_person_character_crazy_people 4)
  (CallFunction|SetSecondaryWeaponEquipped false)
  (CallFunction|SetMeleEquipped false))

(fn OnRepSwichtSecondary
  (CallFunction|SetSecondaryWeaponEquipped true)
  (bind _asbp_third_person_character_crazy_people (Utilities|Casting|CastToBP_ThirdPersonCharacter_CrazyPeople (Variables|Default|GetOwningActor)))
  (Variables|/Game/CrazyPeople/BluePrint/BP_ThirdPersonCharacter_CrazyPeople.BP_ThirdPersonCharacter_CrazyPeople_C|SetTopPoseIndex _asbp_third_person_character_crazy_people 3)
  (CallFunction|SetPrimaryWeaponEquipped false)
  (CallFunction|SetMeleEquipped false))

(fn OnRepSwitchMele
  (CallFunction|SetMeleEquipped true)
  (bind _asbp_third_person_character_crazy_people (Utilities|Casting|CastToBP_ThirdPersonCharacter_CrazyPeople (Variables|Default|GetOwningActor)))
  (Variables|/Game/CrazyPeople/BluePrint/BP_ThirdPersonCharacter_CrazyPeople.BP_ThirdPersonCharacter_CrazyPeople_C|SetTopPoseIndex _asbp_third_person_character_crazy_people 2)
  (CallFunction|SetPrimaryWeaponEquipped false)
  (CallFunction|SetSecondaryWeaponEquipped false))

(fn OnRepIsAiming?)