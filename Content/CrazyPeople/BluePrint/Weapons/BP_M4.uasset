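; BP_M4 is an M4 weapon pickup that player 0's character can equip and drop.
; Overlapping its collision enables input on the weapon and ending the overlap disables it, with no check on which actor overlaps.
; Equip snaps it to the character mesh's HandSocket_R and sets TopPoseIndex on BP_ThirdPersonCharacter_CrazyPeople to the armed pose.
; Drop resets that index and detaches the weapon, keeping its world transform.
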(event OnComponentBeginOverlap(Collition)
  (params (OverlappedComponent :type Primitive%20Component%20Object%20Reference) (OtherActor :type Actor%20Object%20Reference) (OtherComp :type Primitive%20Component%20Object%20Reference) (OtherBodyIndex :type Integer) (bFromSweep :type Boolean) (SweepResult :type Hit%20Result%20Structure%20%28by%20ref%29))
  (Input|EnableInput (Game|GetPlayerController 0)))

(event OnComponentEndOverlap(Collition)
  (params (OverlappedComponent :type Primitive%20Component%20Object%20Reference) (OtherActor :type Actor%20Object%20Reference) (OtherComp :type Primitive%20Component%20Object%20Reference) (OtherBodyIndex :type Integer))
  (Input|DisableInput (Game|GetPlayerController 0)))

(event Input|ActionEvents|InputActionEquip
  (params (Key :type Key%20Structure :default "None"))
  (:Pressed
    (CallFunction|Equip)))

(event Input|ActionEvents|InputActionDrop
  (params (Key :type Key%20Structure :default "None"))
  (:Pressed
    (CallFunction|Drop)))

(fn ConstructionScript)

(fn Equip
  (bind _returnvalue (Game|GetPlayerCharacter 0))
  (Transformation|AttachComponentToComponent (Variables|/Script/Engine.Character|GetMesh _returnvalue) "HandSocket_R" "SnapToTarget" "SnapToTarget" "SnapToTarget" true)
  (bind _asbp_third_person_character_crazy_people (Utilities|Casting|CastToBP_ThirdPersonCharacter_CrazyPeople _returnvalue))
  (Variables|/Game/CrazyPeople/BluePrint/BP_ThirdPersonCharacter_CrazyPeople.BP_ThirdPersonCharacter_CrazyPeople_C|SetTopPoseIndex _asbp_third_person_character_crazy_people 4))

(fn Drop
  (bind _asbp_third_person_character_crazy_people (Utilities|Casting|CastToBP_ThirdPersonCharacter_CrazyPeople (Game|GetPlayerCharacter 0)))
  (Variables|/Game/CrazyPeople/BluePrint/BP_ThirdPersonCharacter_CrazyPeople.BP_ThirdPersonCharacter_CrazyPeople_C|SetTopPoseIndex _asbp_third_person_character_crazy_people 0)
  (Transformation|DetachFromActor "KeepWorld" "KeepWorld" "KeepWorld"))